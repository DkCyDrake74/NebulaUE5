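; BP_MainCamera is a camera actor that pans across the world when the player drags a finger on a touchscreen.
; BeginPlay enables touch events and the DragCamera input records the starting touch location.
; While the first touch is held, Tick moves the actor on the horizontal plane by the frame-to-frame screen delta, swapping axes and negating screen X, without scaling or bounds.
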(event EventBeginPlay
  (Variables|/Script/Engine.PlayerController|SetbEnableTouchEvents (Game|GetPlayerController 0) true))

(event EventTick
  (params (DeltaSeconds :type Float%20%28single-precision%29))
  (bind _returnvalue (Game|GetPlayerController 0))
  (bind (_locationx _locationy _biscurrentlypressed) (Class|PlayerController|GetInputTouchState _returnvalue "Touch1"))
  (if _biscurrentlypressed
    (Variables|Default|SetNewTouchLocation (Math|Vector2D|MakeVector2D _locationx _locationy))
    (Transformation|AddActorWorldOffset (Math|Vector|MakeVector (.y (- (Variables|Default|GetNewTouchLocation) (Variables|Default|GetPreviousTouchLocation))) (* (.x (- (Variables|Default|GetNewTouchLocation) (Variables|Default|GetPreviousTouchLocation))) -1.0) 0.0))
    (Variables|Default|SetPreviousTouchLocation (Variables|Default|GetNewTouchLocation))))

(event Input|ActionEvents|InputActionDragCamera
  (params (Key :type Key%20Structure :default "None"))
  (bind _returnvalue (Game|GetPlayerController 0))
  (bind (_locationx _locationy) (Class|PlayerController|GetInputTouchState _returnvalue "Touch1"))
  (:Pressed
    (Variables|Default|SetPreviousTouchLocation (Math|Vector2D|MakeVector2D _locationx _locationy))))

(fn ConstructionScript)