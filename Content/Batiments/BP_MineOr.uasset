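; BP_MineOr is a gold mine building that accumulates gold over time and shows an info widget when touched.
; Tick drives a Delay that adds BonusGold to its CurrentGold every DelayTime.
; Tick also polls touch input and traces WorldDynamic objects under the cursor; a hit on itself creates WD_MineOr after a short delay.
; Nothing guards against duplicate widgets, so holding the touch keeps adding new ones.
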(event EventTick
  (params (DeltaSeconds :type Float%20%28single-precision%29))
  (bind _returnvalue (Game|GetPlayerController 0))
  (bind _array (Utilities|Array|MakeArray "ObjectTypeQuery2"))
  (bind (_hitresult _returnvalue_2) (Class|PlayerController|GetHitResultUnderCursorforObjects _returnvalue _array true))
  (Utilities|FlowControl|Sequence
    (:then_0
      (Utilities|FlowControl|Delay (Variables|Default|GetDelayTime))
      (Variables|Default|SetCurrentGold (+ (Variables|Default|GetCurrentGold) (Variables|Default|GetBonusGold))))
    (:then_1
      ;[1 1 1] Afficher le widget Info
      (if (.bIsCurrentlyPressed (Class|PlayerController|GetInputTouchState _returnvalue "Touch1"))
        (if _returnvalue_2
          (bind _output_get (Variables|Default|SetHit%20Actor (.HitActor (Collision|BreakHitResult _hitresult))))
          (if (== _output_get self)
            (Utilities|FlowControl|Delay 0.1)
            (bind _returnvalue_3 (UserInterface|CreateWidget "/Game/HUD/Gold/WD_MineOr.WD_MineOr_C"))
            (UserInterface|Viewport|AddtoViewport _returnvalue_3 0)))))))

(fn ConstructionScript)